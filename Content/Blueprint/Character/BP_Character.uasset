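; Top-down player character Blueprint with walk, sprint and aim inputs, a configurable boom camera and test keys for fire and death montages.
; Input flags feed ChangeMovementStates, which delegates to ChangeMovementState.
; Sprinting starts a looping timer that drains SprintDuration, then refills it and clears itself when full.
; Helper functions provide clamped camera zoom, camera shake and facing checks, including a sprint check that reads a separate Stamina variable.
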(event `Key|SpaceBar`
  (params (Key :type "Key Structure"))
  (bind _mesh (`self.Mesh`))
  ;[0.3695 0.9202 1] Test play montage
  (:`Pressed`
    (if (`self.bAimEnabled`)
      (`|PlayMontage` _mesh "/Game/Blueprint/Character/Characters/Mannequin_UE4/Animations/NewFire_Rifle_Ironsights_Montage.NewFire_Rifle_Ironsights_Montage")
      (else
        (`|PlayMontage` _mesh "/Game/Blueprint/Character/Characters/Mannequin_UE4/Animations/NewFire_Rifle_Hip_Montage.NewFire_Rifle_Hip_Montage")))))

(event `Key|V`
  (params (Key :type "Key Structure"))
  ;[0.3695 0.9202 1] Test play montage
  (:`Pressed`
    (`|PlayMontage` (`self.Mesh`) "/Game/Blueprint/Character/Characters/Mannequin_UE4/Animations/NewDeath_1_Montage.NewDeath_1_Montage")))

(event `InputAction|MovementModeChangeWalk`
  (params (Key :type "Key Structure"))
  ;[1 0.5068 0.2107] Движение в зависимости от нажатых кнопок
  (:`Pressed`
    (set `self.bWalkEnabled` true)
    (`self.Change Movement States` :!label _label))
  (:`Released`
    (set `self.bWalkEnabled` false)
    (goto _label)))

(event `StaminaTick`
  ;[1 0.2731 0.5816] Активация стамины по таймеру
  (if (and (`self.bSprintRunEnabled`) (> (`self.SprintDuration`) 0.0))
    (bind _output_get (set `self.SprintDuration` (- (`self.SprintDuration`) 10.0)))
    (if (<= _output_get 0.0)
      (set `self.SprintDuration` 0.0)
      (set `self.bSprintRunEnabled` false)
      (`self.Change Movement States`)
      (`KismetSystemLibrary.PrintString` (`KismetStringLibrary.Conv_DoubleToString` _output_get)))
    (else
      (set `self.bSprintRunEnabled` false)
      (`self.Change Movement States`)
      (bind _output_get_2 (set `self.SprintDuration` (+ (`self.SprintDuration`) 5.0)))
      (if (>= _output_get_2 100.0)
        (`KismetSystemLibrary.K2_ClearAndInvalidateTimerHandle` (`self.StaminaTimer`))
        (bind _output_get_3 (set `self.SprintDuration` 100.0))
        (`KismetSystemLibrary.PrintString` (`KismetStringLibrary.Conv_DoubleToString` _output_get_3))))))

(event `InputAction|MovementModeChangeSprint`
  (params (Key :type "Key Structure"))
  ;[1 0.5068 0.2107] Движение в зависимости от нажатых кнопок
  (:`Pressed`
    (set `self.bSprintRunEnabled` true)
    (`|ExecutionSequence`
      (:`then_0`
        ;[1 0.2731 0.5816] Активация стамины по таймеру
        (bind _returnvalue (`KismetSystemLibrary.K2_SetTimerDelegate` (delegate `StaminaTick`) 1.0 true))
        (set `self.StaminaTimer` _returnvalue)
        (`self.StaminaTick`))
      (:`then_1`
        (goto _label))))
  (:`Released`
    (set `self.bSprintRunEnabled` false)
    (goto _label)))

(event `Key|RightMouseButton`
  (params (Key :type "Key Structure"))
  ;[1 0.5068 0.2107] Движение в зависимости от нажатых кнопок
  (:`Pressed`
    (set `self.bAimEnabled` true)
    (goto _label))
  (:`Released`
    (set `self.bAimEnabled` false)
    (goto _label)))

(fn `CameraShakeEvent`
  ;[1 0.6299 0.468] Тряска камеры
  (`GameplayStatics.PlayWorldCameraShake` "/Game/Blueprint/Game/BP_ShakeCamera.BP_ShakeCamera_C" (`SceneComponent.K2_GetComponentLocation` (`self.TopDownCameraComponent`)) 0.0 30.0))

(fn `CameraSlide`
  (params (Value :type "Float (double-precision)"))
  (bind _cameraboom (`self.CameraBoom`))
  ;[1 0.1401 0.1301] Упрощенная работа функции CameraSlide
  (bind _output_get (set `self.Height` (`KismetMathLibrary.FClamp` (- (`self.Height`) (* Value 40.0)) 50.0 1200.0)))
  (set `SpringArmComponent.TargetArmLength` (`KismetMathLibrary.FInterpTo` (`SpringArmComponent.TargetArmLength` _cameraboom) _output_get (`GameplayStatics.GetWorldDeltaSeconds`)) _cameraboom))

(fn `Can Sprinting`
  (returns (ReturnValue :type Boolean))
  ;[1 0.8739 0.6936] Ограничения по направлению бега
  (return (and (> (`KismetMathLibrary.Dot_VectorVector` (`KismetMathLibrary.Normal` (`KismetMathLibrary.MakeVector` (.x (`self.GetVelocity`)) (.y (`self.GetVelocity`)))) (`self.GetActorForwardVector`)) (`self.SprintLookTolerance`)) (>= (`self.Stamina`) (`self.DiscriseStaminaValue`)))))

(fn `Change Movement States`
  (`self.ChangeMovementState`))

(fn `CheckCorrectRotation`
  (returns (ReturnValue :type Boolean))
  (bind (_returnvalue_x _returnvalue_y) (`KismetMathLibrary.BreakVector` (`self.GetLastMovementInputVector`)))
  (bind (_returnvalue_x_2 _returnvalue_y_2) (`KismetMathLibrary.BreakVector` (`KismetMathLibrary.GetForwardVector` (`self.K2_GetActorRotation`))))
  (return (and (>= (* _returnvalue_y_2 _returnvalue_y) 0.0) (>= (* _returnvalue_x_2 _returnvalue_x) 0.0))))

(fn `IsMovingForward`
  (returns (ReturnValue :type Boolean))
  (return (<= (`KismetMathLibrary.DegAcos` (`KismetMathLibrary.Dot_VectorVector` (`self.GetActorForwardVector`) (`KismetMathLibrary.Normal` (`self.GetVelocity`)))) 10.0)))

(fn `UserConstructionScript`
  (bind _cameraboom (`self.CameraBoom`))
  ;[0.4366 1 0.8694] Ротация по курсору
  (set `SpringArmComponent.TargetArmLength` (`self.Hieght`) _cameraboom)
  (`SceneComponent.K2_SetRelativeRotation` _cameraboom (`self.RotatorCamera`) false false)
  (set `SpringArmComponent.bEnableCameraLag` (`self.Flow`) _cameraboom)
  (set `SpringArmComponent.CameraLagSpeed` (`self.CoefSmooth`) _cameraboom))